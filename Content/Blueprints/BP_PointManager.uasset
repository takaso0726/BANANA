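; BP_PointManager is a score manager that keeps running totals for three point types: humor, color and flame (online backlash).
; On BeginPlay it creates the WBP_UI widget and adds it to the viewport.
; AddScore adds each incoming value to its total and passes all three totals in sequence to the same ApplyScore call on the widget, with flame last.
; It also prints a "Hello" debug string.
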(event EventBeginPlay
  (bind _returnvalue (UserInterface|CreateWidget "/Game/Widget/WBP_UI.WBP_UI_C"))
  (bind _output_get (Variables|Default|SetgameUI _returnvalue))
  (UserInterface|Viewport|AddtoViewport _output_get 0))

(event EventTick
  (params (DeltaSeconds :type Float%20%28single-precision%29)))

(fn ConstructionScript)

(fn AddScore
  (params (Humor :type Integer) (Color :type Integer) (Frame :type Integer))
  (Development|PrintString "Hello")
  (Utilities|FlowControl|Sequence
    (:then_0
      ;[0.15 0.15 0.15 0.5] ユーモアの合計点
      (bind _output_get (Variables|Default|SetTotalHumor (+ (Variables|Default|GetTotalHumor) Humor)))
      (Default|ApplyScore (Variables|Default|GetgameUI) _output_get))
    (:then_1
      ;[0.15 0.15 0.15 0.5] カラーの合計点
      (bind _output_get_2 (Variables|Default|SetTotalColor (+ (Variables|Default|GetTotalColor) Color)))
      (Default|ApplyScore (Variables|Default|GetgameUI) _output_get_2))
    (:then_2
      ;[0.15 0.15 0.15 0.5] 炎上の合計点
      (bind _output_get_3 (Variables|Default|SetTotalFlame (+ (Variables|Default|GetTotalFlame) Frame)))
      (Default|ApplyScore (Variables|Default|GetgameUI) _output_get_3))))