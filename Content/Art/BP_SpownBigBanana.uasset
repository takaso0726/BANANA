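; Actor Blueprint that grows its Banana component from a start scale to a target scale when it spawns.
; BeginPlay starts the growth timer, and Tick accumulates delta time to lerp the relative scale until GrowTime is reached, then clears IsGrowing.
; Several disconnected leftover chains for debug printing, movement, incremental scaling and alpha setting never run.
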(event EventBeginPlay
  (Variables|Default|SetIsGrowing true)
  (Variables|Default|SetCurrentGrowTime 0.0)
  (Variables|Default|SetStartScale (Variables|Default|GetStartScale)))

(event EventTick
  (params (DeltaSeconds :type Float%20%28single-precision%29))
  (Utilities|FlowControl|Sequence
    (:then_0
      (if (Variables|Default|GetIsGrowing)
        (Variables|Default|SetCurrentGrowTime (+ (Variables|Default|GetCurrentGrowTime) (Utilities|Time|GetWorldDeltaSeconds)))
        (Transformation|SetRelativeScale3D (Variables|Default|GetBanana) (Math|Vector|Lerp(Vector) (Variables|Default|GetStartScale) (Variables|Default|GetTargetScale) (/ (Variables|Default|GetCurrentGrowTime) (Variables|Default|GetGrowTime))))))
    (:then_1
      (if (>= (Variables|Default|GetCurrentGrowTime) (Variables|Default|GetGrowTime))
        (Variables|Default|SetIsGrowing false)))))

(fn ConstructionScript)