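; BP_Banana is a banana projectile actor with a short lifespan and a ProjectileMovement component driven by LaunchSpeed.
; On BeginPlay it computes a suggested toss velocity toward a fixed point from its scaled location, but uses that vector only as an emitter's spawn location.
; Overlapping an actor tagged "meiga" lengthens its lifespan and prints a hit message.
; A 2D sound call is present but never runs.
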(event OnComponentBeginOverlap(banana)
  (params (OverlappedComponent :type Primitive%20Component%20Object%20Reference) (OtherActor :type Actor%20Object%20Reference) (OtherComp :type Primitive%20Component%20Object%20Reference) (OtherBodyIndex :type Integer) (bFromSweep :type Boolean) (SweepResult :type Hit%20Result%20Structure%20%28by%20ref%29))
  (if (Actor|ActorHasTag OtherActor "meiga")
    (Actor|SetLifeSpan 5e+01)
    (Development|PrintText "hit!!")))

(event EventBeginPlay
  (bind _projectilemovement (Variables|Default|GetProjectileMovement))
  (bind _launchspeed (Variables|Default|GetLaunchSpeed))
  (Actor|SetLifeSpan 5.0)
  (Variables|/Script/Engine.ProjectileMovementComponent|SetMaxSpeed _projectilemovement _launchspeed)
  (bind _output_get (Variables|/Script/Engine.ProjectileMovementComponent|SetInitialSpeed _projectilemovement _launchspeed))
  (bind _tossvelocity (Class|GameplayStatics|BlueprintSuggestProjectileVelocity (* (Transformation|GetActorLocation) 5e+01) "2000.000000,0.000000,0.000000" _output_get 1.0 "DoNotTrace" 0.0 false false false))
  (Effects|SpawnEmitteratLocation 0 _tossvelocity))

(fn ConstructionScript)