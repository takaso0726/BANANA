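; BP_Painting3 is a painting actor that awards score when a BP_Banana overlaps one of its three hit boxes.
; On BeginPlay it caches the level's BP_PointManager.
; HumorBox, ColorBox and FlameBox each call the manager's AddScore with their own value in the matching category, with FlameBox feeding Frame.
; Debug prints report each hit and a missing manager, though "ManagerFound" prints without a validity check.
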(event OnComponentBeginOverlap(HumorBox)
  (params (OverlappedComponent :type Primitive%20Component%20Object%20Reference) (OtherActor :type Actor%20Object%20Reference) (OtherComp :type Primitive%20Component%20Object%20Reference) (OtherBodyIndex :type Integer) (bFromSweep :type Boolean) (SweepResult :type Hit%20Result%20Structure%20%28by%20ref%29))
  (Utilities|Casting|CastToBP_Banana OtherActor)
  (Development|PrintString "Humor")
  (Utilities|IsValid (Variables|Default|GetPointManagerRef)
    (:Is%20Valid
      (Development|PrintString (Variables|Default|GetPaintingName))
      (Default|AddScore (Variables|Default|GetPointManagerRef) (Variables|Default|GetHumorValue))
      (Development|PrintString (Utilities|String|ToString(Integer) (Variables|Default|GetHumorValue))))
    (:Is%20Not%20Valid
      (Development|PrintString "Manager NULL"))))

(event OnComponentBeginOverlap(FlameBox)
  (params (OverlappedComponent :type Primitive%20Component%20Object%20Reference) (OtherActor :type Actor%20Object%20Reference) (OtherComp :type Primitive%20Component%20Object%20Reference) (OtherBodyIndex :type Integer) (bFromSweep :type Boolean) (SweepResult :type Hit%20Result%20Structure%20%28by%20ref%29))
  (Utilities|Casting|CastToBP_Banana OtherActor)
  (Development|PrintString "Flame")
  (Utilities|IsValid (Variables|Default|GetPointManagerRef)
    (:Is%20Valid
      (Development|PrintString "Manager OK")
      (Default|AddScore (Variables|Default|GetPointManagerRef) 0 0 (Variables|Default|GetFlameValue)))
    (:Is%20Not%20Valid
      (Development|PrintString "Manager NULL"))))

(event OnComponentBeginOverlap(ColorBox)
  (params (OverlappedComponent :type Primitive%20Component%20Object%20Reference) (OtherActor :type Actor%20Object%20Reference) (OtherComp :type Primitive%20Component%20Object%20Reference) (OtherBodyIndex :type Integer) (bFromSweep :type Boolean) (SweepResult :type Hit%20Result%20Structure%20%28by%20ref%29))
  (Utilities|Casting|CastToBP_Banana OtherActor)
  (Development|PrintString "Color")
  (Utilities|IsValid (Variables|Default|GetPointManagerRef)
    (:Is%20Valid
      (Development|PrintString "Manager OK")
      (Default|AddScore (Variables|Default|GetPointManagerRef) 0 (Variables|Default|GetColorValue)))
    (:Is%20Not%20Valid
      (Development|PrintString "Manager NULL"))))

(event EventBeginPlay
  (bind _returnvalue (Actor|GetActorOfClass "/Game/Blueprints/BP_PointManager.BP_PointManager_C"))
  (Variables|Default|SetPointManagerRef _returnvalue)
  (Development|PrintString "ManagerFound"))

(fn ConstructionScript)