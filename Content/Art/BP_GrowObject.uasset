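; BP_GrowObject is a cube actor that grows each time a BP_Banana overlaps its action box, up to a maximum count.
; Each step scales the mesh from its initial size, raises the actor, and enlarges and shifts the hitbox to match.
; On the final step it spawns a BP_SpownBigBanana at the spawn point.
; A debug G key, enabled through player input on BeginPlay, triggers the same growth.
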(event OnComponentBeginOverlap(actionbox)
  (params (OverlappedComponent :type Primitive%20Component%20Object%20Reference) (OtherActor :type Actor%20Object%20Reference) (OtherComp :type Primitive%20Component%20Object%20Reference) (OtherBodyIndex :type Integer) (bFromSweep :type Boolean) (SweepResult :type Hit%20Result%20Structure%20%28by%20ref%29))
  (Utilities|Casting|CastToBP_Banana OtherActor)
  (CallFunction|GrowObject))

(event Custom|GrowObject
  (bind _returnvalue (Transformation|GetActorLocation))
  (bind (_x _y _z) (Math|Vector|BreakVector _returnvalue))
  (if (< (Variables|Default|GetCurrentScaleCount) (Variables|Default|GetMaxScaleCount))
    (Variables|Default|SetCurrentScaleCount (+ (Variables|Default|GetCurrentScaleCount) 1))
    (Transformation|SetRelativeScale3D (Variables|Default|GetSM_Cube) (+ (Variables|Default|GetInitialScale) (Math|Vector|MakeVector (* (Variables|Default|GetCurrentScaleCount) (Variables|Default|GetScaleUpAmount)) (* (Variables|Default|GetCurrentScaleCount) (Variables|Default|GetScaleUpAmount)) (* (Variables|Default|GetCurrentScaleCount) (Variables|Default|GetScaleUpAmount)))))
    (Transformation|SetActorLocation (Math|Vector|MakeVector _x _y (+ _z 2e+01)) false false)
    ;[0.15 0.15 0.15 0.5] hitboxを大きく
    (Components|Box|SetBoxExtent (Variables|Default|Getactionbox) (+ (Components|Box|GetUnscaledBoxExtent (Variables|Default|Getactionbox)) (Math|Vector|MakeVector 2e+01 2e+01 2e+01)) true)
    ;[0.15 0.15 0.15 0.5] hitboxを上に
    (Transformation|SetRelativeLocation (Variables|Default|Getactionbox) (+ (.Location (Math|Transform|BreakTransform (Transformation|GetRelativeTransform (Variables|Default|Getactionbox)))) (Math|Vector|MakeVector 5.0 0.0 1e+01)) false false)
    ;[0.15 0.15 0.15 0.5] 回数がマックス
    (if (== (Variables|Default|GetCurrentScaleCount) (Variables|Default|GetMaxScaleCount))
      ;[0.15 0.15 0.15 0.5] バナナを出す
      (Game|SpawnActorfromClass "/Game/Art/BP_SpownBigBanana.BP_SpownBigBanana_C" (Transformation|GetWorldTransform (Variables|Default|GetSpawnPoint)) "Undefined" "MultiplyWithRoot" 0 0))))

(event EventBeginPlay
  (Input|EnableInput (Game|GetPlayerController 0))
  (Variables|Default|SetInitialScale (Variables|/Script/Engine.SceneComponent|GetRelativeScale3D (Variables|Default|GetSM_Cube))))

(event Input|KeyboardEvents|DebugKeyG
  (params (Key :type Key%20Structure) (ActionValue :type Input%20Action%20Value%20Structure))
  (:Pressed
    (CallFunction|GrowObject)))

(fn ConstructionScript)